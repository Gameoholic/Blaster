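; Widget component for the lobby settings menu, where a map is selected and the game is started.
; On BeginPlay it caches its WBP_LobbySettings widget, supplies the map list and binds the start and map button events.
; Button clicks pass through wrapper functions to StartGame and SelectMap, which are defined outside these graphs.
; When SelectedMapPath replicates, OnReplicatedSelectedMapPath pushes it back to the widget.
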(event Custom|StartButtonClickedEvent
  ;[0.5569 1 0.3338] Set up StartButtonClicked Event Listener
  (CallFunction|StartButtonClicked))

(event Custom|MapButtonClickedEvent
  (params (SelectedMapPathString :type String))
  ;[0.5569 1 0.3338] Set up MapButtonClicked Event Listener
  (CallFunction|MapButtonClicked SelectedMapPathString))

(event EventBeginPlay
  ;[1 1 1] WBP_LobbySettings
  (bind _aswbp_lobby_settings (Utilities|Casting|CastToWBP_LobbySettings (UserInterface|GetUserWidgetObject)))
  (bind _output_get (Variables|Default|SetWBP_LobbySettings _aswbp_lobby_settings))
  (Default|SetMaps _output_get (Variables|Default|GetMaps))
  ;[0.5569 1 0.3338] Set up StartButtonClicked Event Listener
  (EventDispatchers|BindEventtoStartButtonClicked (Variables|Default|GetWBP_LobbySettings) (delegate Custom|StartButtonClickedEvent))
  ;[0.5569 1 0.3338] Set up MapButtonClicked Event Listener
  (EventDispatchers|BindEventtoMapButtonClicked (Variables|Default|GetWBP_LobbySettings) (delegate Custom|MapButtonClickedEvent)))

(event EventOnReplicatedSelectedMapPath
  (Default|OnSelectedMapReplicated (Variables|Default|GetWBP_LobbySettings) (Variables|Default|GetSelectedMapPath)))

(fn StartButtonClicked
  (Class|LobbySettingsWidgetComponent|StartGame))

(fn MapButtonClicked
  (params (SelectedMapPathString :type String))
  (Class|LobbySettingsWidgetComponent|SelectMap SelectedMapPathString))