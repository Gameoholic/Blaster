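; Player character Blueprint for Blaster that adds a starting weapon, sniper scope feedback and a temporary fall-death check.
; On BeginPlay it spawns and force-equips an assault rifle, only when the game mode is BlasterGameMode, which excludes the lobby.
; The scope event lazily creates its widget, playing one zoom animation forward or reversed with matching sounds.
; Tick reports the player killed to the game mode below a Z threshold.
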(event EventBeginPlay
  (CallFunction|SpawnandEquipWeapon))

(event EventShowSniperScopeWidget
  (params (bShowScope :type Boolean))
  ;[1 1 1] Sniper scope widget event implementation
  (Utilities|IsValid (Variables|Default|GetSniperScopeWidget)
    (:Is%20Valid
      _)
    (:Is%20Not%20Valid
      (bind _returnvalue (UserInterface|CreateWidget "/Game/Blueprints/HUD/WBP_SniperScope.WBP_SniperScope_C"))
      (Utilities|IsValid _returnvalue
        (:Is%20Valid
          (bind _output_get (Variables|Default|SetSniperScopeWidget _returnvalue))
          (UserInterface|Viewport|AddtoViewport _output_get 0)))))
  (if bShowScope
    (UserInterface|Animation|PlayAnimation (Variables|Default|GetSniperScopeWidget) (Variables|/Game/Blueprints/HUD/WBP_SniperScope.WBP_SniperScope_C|GetScopeZoomIn (Variables|Default|GetSniperScopeWidget)) 0.0 1 "Forward" 1.0 false)
    (Audio|PlaySound2D "/Game/Assets/MilitaryWeapSilver/Sound/SniperRifle/Cues/SniperRifle_ZoomIn_Cue.SniperRifle_ZoomIn_Cue" 1.0 1.0 0.0 0 0)
    (else
      (UserInterface|Animation|PlayAnimation (Variables|Default|GetSniperScopeWidget) (Variables|/Game/Blueprints/HUD/WBP_SniperScope.WBP_SniperScope_C|GetScopeZoomIn (Variables|Default|GetSniperScopeWidget)) 0.0 1 "Reverse" 1.0 false)
      (Audio|PlaySound2D "/Game/Assets/MilitaryWeapSilver/Sound/SniperRifle/Cues/SniperRifle_ZoomOut_Cue.SniperRifle_ZoomOut_Cue" 1.0 1.0 0.0 0 0))))

(event EventTick
  (params (DeltaSeconds :type Float%20%28single-precision%29))
  ;[1 0 0] Kill player if fall from map (TEMPORARY)
  (if (<= (.z (Transformation|GetActorLocation)) -2.5e+03)
    (bind _asblaster_game_mode (Utilities|Casting|CastToBlasterGameMode (Game|GetGameMode)))
    (bind _asblaster_player_controller (Utilities|Casting|CastToBlasterPlayerController (Pawn|GetController self)))
    (Class|BlasterGameMode|PlayerKilled _asblaster_game_mode self _asblaster_player_controller)))

(event Input|KeyboardEvents|F
  (params (Key :type Key%20Structure :default "None")))

(fn ConstructionScript)

(fn SpawnandEquipWeapon
  ;[1 1 1] Only if not in lobby
  (Utilities|Casting|CastToBlasterGameMode (Game|GetGameMode))
  (bind _returnvalue (Game|SpawnActorfromClass "/Game/Blueprints/Weapon/BP_AssaultRifle.BP_AssaultRifle_C" (Math|Transform|MakeTransform (Math|Vector|MakeVector 0.0 0.0 0.0) "0, 0, 0" "1.000000,1.000000,1.000000") "AdjustIfPossibleButAlwaysSpawn" "MultiplyWithRoot" 0 self))
  (Class|BlasterCharacter|ForceEquipWeapon _returnvalue))